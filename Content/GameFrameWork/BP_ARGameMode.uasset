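; BP_ARGameMode is the AR game mode that switches the game state between sports ball types and spawns balls.
; ChangeStateByName maps a ball name to a sport state, passes it to BP_ARGameState's ChangeState, then spawns a BP_Ball given that name.
; GetCurrentGameState reads the current state from the game state.
; The event graph contains only an unconnected switch on that state.
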(fn ConstructionScript)

(fn ChangeStatebyName
  (params (BalllName :type Name))
  (Utilities|FlowControl|Sequence
    (:then_0
      (switch name BalllName
        (:Baseball
          (LocalVariables|SetNewState "NewEnumerator1"))
        (:Basketball
          (LocalVariables|SetNewState "NewEnumerator2"))
        (:Football
          (LocalVariables|SetNewState "NewEnumerator3"))
        (:Golf
          (LocalVariables|SetNewState "NewEnumerator4"))
        (:Soccor
          (LocalVariables|SetNewState "NewEnumerator5"))
        (:Tennis
          (LocalVariables|SetNewState "NewEnumerator6"))
        (:Volleyball
          (LocalVariables|SetNewState "NewEnumerator7"))))
    (:then_1
      (bind _asbp_argame_state (Utilities|Casting|CastToBP_ARGameState (Game|GetGameState)))
      (Default|ChangeState _asbp_argame_state (LocalVariables|GetNewState))
      (Game|SpawnActorfromClass "/Game/Placeable/BP_Ball.BP_Ball_C" (Math|Transform|MakeTransform "0, 0, 0" "0, 0, 0" "1.000000,1.000000,1.000000") "Undefined" "MultiplyWithRoot" 0 BalllName 0))))

(fn GetCurrentGameState
  (bind _asbp_argame_state (Utilities|Casting|CastToBP_ARGameState (Game|GetGameState)))
  (return (Variables|/Game/GameFrameWork/BP_ARGameState.BP_ARGameState_C|GetCurrentState _asbp_argame_state)))