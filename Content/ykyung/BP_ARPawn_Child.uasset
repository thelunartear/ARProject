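; AR pawn child Blueprint that throws a basketball when F is pressed.
; The key spawns a BP_Ball1 offset from the camera, then applies a velocity-change impulse to its mesh.
; Horizontal impulse follows the camera's aim scaled by ThrowPower, while vertical impulse is remapped from aim pitch with a fixed multiplier to add loft.
; After each throw, the pawn's rotation snaps to the control rotation.
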(event EventBeginPlay)

(event Collision|EventActorBeginOverlap
  (params (OtherActor :type Actor%20Object%20Reference)))

(event EventTick
  (params (DeltaSeconds :type Float%20%28single-precision%29))
  (|CallParentFunction DeltaSeconds))

(event Input|KeyboardEvents|F
  (params (Key :type Key%20Structure :default "None"))
  (bind _returnvalue (Game|GetPlayerCameraManager 0))
  (bind _camera (Variables|Default|GetCamera))
  (bind _throwpower (Variables|Default|GetThrowPower))
  (bind _returnvalue_2 (Camera|GetCameraRotation _returnvalue))
  (bind _returnvalue_3 (Math|Vector|GetForwardVector _returnvalue_2))
  (bind _returnvalue_4 (* _returnvalue_3 _throwpower))
  (bind (_x _y) (Math|Vector|BreakVector _returnvalue_4))
  (:Pressed
    (bind _returnvalue_5 (Game|SpawnActorfromClass "/Game/ykyung/BP_Ball1.BP_Ball1_C" (Math|Transform|MakeTransform (+ (+ (Transformation|GetWorldLocation _camera) (Variables|Default|GetSpawnOffsetDist)) (* (Math|Vector|GetForwardVector _camera) (Variables|Default|GetSpawnOffsetDist))) "0, 0, 0" "1.000000,1.000000,1.000000") "Undefined" "MultiplyWithRoot" 0 "BasketBall" 0))
    (Physics|AddImpulse (Variables|/Game/ykyung/BP_Ball1.BP_Ball1_C|GetStaticMesh _returnvalue_5) (Math|Vector|MakeVector _x _y (* (Math|Float|MapRangeUnclamped (.Z (Math|Vector|BreakVector _returnvalue_3)) 0.0 1.0 3.0 1e+01) 5e+02)) "None" true)
    (Transformation|SetActorRotation (Pawn|GetControlRotation :!class /Script/Engine.Pawn))))

(fn ConstructionScript
  (|CallParentFunction))