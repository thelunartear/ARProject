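; BP_Ball is a placeable ball actor that sets itself up from data and drops into the level as a physics object.
; On BeginPlay it looks up its Name in DT_Balls, applies that row's mesh, and adjusts the component's relative location and rotation using the mesh's "Root" socket.
; It then moves itself slightly above the BP_Plane actor found in the level and enables physics simulation.
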(event EventBeginPlay
  (bind _staticmesh (Variables|Default|GetStaticMesh))
  (bind _staticmesh_2 (Variables|Default|GetStaticMesh))
  (bind _returnvalue (Utilities|GetDataTableRow "/Game/Placeable/Balls/DT_Balls.DT_Balls" (Variables|Default|GetName))
    (:then
      (Components|StaticMesh|SetStaticMesh (Variables|Default|GetStaticMesh) (.Mesh (Utilities|Struct|BreakST_Balls _returnvalue)))
      (Transformation|AddRelativeLocation _staticmesh (* -1.0 (Transformation|GetSocketLocation _staticmesh "Root")) false false)
      (Transformation|AddRelativeRotation _staticmesh_2 (Transformation|GetSocketRotation _staticmesh_2 "Root") false false)
      (bind _returnvalue_2 (Actor|GetActorOfClass "/Game/Placeable/BP_Plane.BP_Plane_C"))
      (Transformation|SetActorLocation (+ (Transformation|GetActorLocation _returnvalue_2) "0.000000,0.000000,50.000000") false false)
      (Physics|SetSimulatePhysics (Variables|Default|GetStaticMesh) true))))

(fn ConstructionScript)