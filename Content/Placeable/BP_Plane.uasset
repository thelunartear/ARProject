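; BP_Plane is a placeable AR court with invisible walls that keep the ball in bounds and a sport-selection widget.
; CheckSize rates the floor's scale into size tiers, and ShowWidget adds the sports that fit, from Baseball up to Golf.
; The widget turns toward the camera each tick.
; On game-state changes it moves to the bottom of the screen in one state and leaves the viewport in most others.
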(event Custom|CheckState
  ;[0.15 0.15 0.15 0.5] 위젯을 제거하고 UI에 띄움
  (CallFunction|MoveWidgettoViewport))

(event EventBeginPlay
  ;[0.15 0.15 0.15 0.5] 벽 투명화(공 범위 제한)
  (Rendering|SetVisibility (Variables|Default|GetWallFront) false false)
  ;[0.15 0.15 0.15 0.5] 상태 변경 감지
  (bind _asbp_argame_state (Utilities|Casting|CastToBP_ARGameState (Game|GetGameState)))
  (EventDispatchers|BindEventtoDispatcherStateChanged _asbp_argame_state (delegate Custom|CheckState)))

(event EventTick
  (params (DeltaSeconds :type Float%20%28single-precision%29))
  (bind _widget (Variables|Default|GetWidget))
  ;[0.15 0.15 0.15 0.5] 위젯이 카메라 바라보게 하는 용도
  (Transformation|SetWorldRotation _widget (Math|Rotator|FindLookatRotation (Transformation|GetWorldLocation _widget) (Transformation|GetActorLocation (Game|GetPlayerCameraManager 0))) false false))

(fn ConstructionScript)

(fn CheckSize
  (bind _floor (Variables|Default|GetFloor))
  (bind _relativescale3d (Variables|/Script/Engine.SceneComponent|GetRelativeScale3D _floor))
  (Utilities|FlowControl|Sequence
    (:then_0
      (LocalVariables|SetMaxVar (Math|Float|Max(Float) (.x _relativescale3d) (.y _relativescale3d)))
      (LocalVariables|SetMinVar (Math|Float|Min(Float) (.x _relativescale3d) (.y _relativescale3d)))
      (Variables|Default|SetbIsWidthLonger (> (.x _relativescale3d) (.y _relativescale3d)))
      (Variables|Default|SetSizeOfCourt 0))
    (:then_1
      (if (and (> (LocalVariables|GetMaxVar) 1.0) (> (LocalVariables|GetMinVar) 1.0))
        (Math|Integer|IncrementInt (Variables|Default|GetSizeOfCourt))))
    (:then_2
      (if (and (> (LocalVariables|GetMaxVar) 1e+01) (> (LocalVariables|GetMinVar) 5.0))
        (Math|Integer|IncrementInt (Variables|Default|GetSizeOfCourt))))
    (:then_3
      (if (and (> (LocalVariables|GetMaxVar) 16.0) (> (LocalVariables|GetMinVar) 8.0))
        (Math|Integer|IncrementInt (Variables|Default|GetSizeOfCourt))))
    (:then_4
      (if (and (> (LocalVariables|GetMaxVar) 2e+01) (> (LocalVariables|GetMinVar) 2e+01))
        (Math|Integer|IncrementInt (Variables|Default|GetSizeOfCourt))))
    (:then_5
      (CallFunction|ShowWidget))))

(fn ShowWidget
  (bind _asselect_widget (Utilities|Casting|CastToSelectWidget (UserInterface|GetWidget (Variables|Default|GetWidget))))
  (LocalVariables|SetItsWidget _asselect_widget)
  (for _index (range 0 (Variables|Default|GetSizeOfCourt))
    (switch int _index
      (:1
        (Default|AddItem (LocalVariables|GetItsWidget) "Baseball")
        (Default|AddItem (LocalVariables|GetItsWidget) "Basketball"))
      (:2
        (Default|AddItem (LocalVariables|GetItsWidget) "Tennis")
        (Default|AddItem (LocalVariables|GetItsWidget) "Volleyball"))
      (:3
        (Default|AddItem (LocalVariables|GetItsWidget) "Football")
        (Default|AddItem (LocalVariables|GetItsWidget) "Soccor"))
      (:4
        (Default|AddItem (LocalVariables|GetItsWidget) "Golf"))))
  (return))

(fn MoveWidgettoViewport
  (bind _returnvalue (Viewport|GetViewportSize))
  (bind _widget (Variables|Default|GetWidget))
  (bind _returnvalue_2 (UserInterface|GetWidget _widget))
  (bind _asbp_argame_state (Utilities|Casting|CastToBP_ARGameState (Game|GetGameState)))
  (if (Utilities|Enum|Equal(Enum) (Variables|/Game/GameFrameWork/BP_ARGameState.BP_ARGameState_C|GetCurrentState _asbp_argame_state) "NewEnumerator8")
    (UserInterface|Viewport|AddtoViewport _returnvalue_2 0)
    (Widget|Transform|SetRenderScale _returnvalue_2 "(X=2.000000,Y=2.000000)")
    (Class|UserWidget|SetAlignmentinViewport _returnvalue_2 (Math|Vector2D|MakeVector2D 0.5 0.5))
    (Class|UserWidget|SetPositioninViewport _returnvalue_2 (Math|Vector2D|MakeVector2D (/ (.x _returnvalue) 2.0) (- (.y _returnvalue) 1e+02)) true)
    (Rendering|SetVisibility (Variables|Default|GetWidget) false false)
    (elif (Utilities|Enum|NotEqual(Enum) (Variables|/Game/GameFrameWork/BP_ARGameState.BP_ARGameState_C|GetCurrentState _asbp_argame_state) "NewEnumerator0")
      (Widget|RemovefromParent _returnvalue_2))))